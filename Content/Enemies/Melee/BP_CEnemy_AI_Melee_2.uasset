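; BP_CEnemy_AI_Melee_2 is a melee enemy Blueprint whose own graphs contain no active logic.
; Tick, ShowHitNumber and the construction script are empty.
; Disconnected nodes hold an unused floating damage-number routine that projects the hit location to screen, stores a WB_CHitNumber widget and plays its animation, plus a montage debug print.
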(event EventTick
  (params (DeltaSeconds :type Float%20%28single-precision%29)))

(event EventShowHitNumber
  (params (InDamage :type Integer) (InHitLocation :type Vector :default "0, 0, 0")))

(fn ConstructionScript)